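; STGAsteroid is an asteroid actor that drifts in a random horizontal direction while spinning.
; The construction script projects a random unit vector onto the XY plane and normalizes it as the ProjectileMovement velocity, with MovementSpeed setting both initial and max speed.
; Tick yaws the InstancedStaticMesh component locally by RotationSpeed scaled by delta time, for a frame-rate-independent spin.
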(event EventBeginPlay)

(event Collision|EventActorBeginOverlap
  (params (OtherActor :type Actor%20Object%20Reference)))

(event EventTick
  (params (DeltaSeconds :type Float%20%28single-precision%29))
  (Transformation|AddLocalRotation (Variables|Default|GetInstancedStaticMesh) (Math|Rotator|MakeRotator 0.0 0.0 (* DeltaSeconds (Variables|Default|GetRotationSpeed))) false false))

(fn ConstructionScript
  (bind _projectilemovement (Variables|Default|GetProjectileMovement))
  (bind _movementspeed (Variables|Default|GetMovementSpeed))
  (Variables|/Script/Engine.MovementComponent|SetVelocity _projectilemovement (Math|Vector|Normalize (Math|Vector|ProjectVectorontoPlane (Math|Random|RandomUnitVector) "0, 0,1.000000")))
  (Variables|/Script/Engine.ProjectileMovementComponent|SetInitialSpeed _projectilemovement _movementspeed)
  (Variables|/Script/Engine.ProjectileMovementComponent|SetMaxSpeed _projectilemovement _movementspeed))