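; STGHud is the HUD Blueprint that shows the owning player's score, hits and kills on screen.
; On BeginPlay it creates a HUD widget for the owning player controller and adds it to the viewport.
; Every Tick it casts the PlayerState to STGPlayerState and pushes Hits and Kills into the widget.
; Score is derived on the fly by a math expression that weights kills more heavily than hits.
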(event EventBeginPlay
  (bind _returnvalue (UserInterface|CreateWidget "/Game/UI/HUD.HUD_C" (Game|Player|GetOwningPlayerController)))
  (bind _output_get (Variables|Default|SetHUD _returnvalue))
  (UserInterface|Viewport|AddtoViewport _output_get 0))

(event Collision|EventActorBeginOverlap
  (params (OtherActor :type Actor%20Object%20Reference)))

(event EventTick
  (params (DeltaSeconds :type Float%20%28single-precision%29))
  (bind _hud (Variables|Default|GetHUD))
  (bind _asstgplayer_state (Utilities|Casting|CastToSTGPlayerState (Variables|/Script/Engine.Controller|GetPlayerState (Game|Player|GetOwningPlayerController))))
  (Utilities|FlowControl|Sequence
    (:then_0
      (Variables|/Game/UI/HUD.HUD_C|SetScore _hud (|((hits*1111)+(kills*5555)) (Variables|/Game/Blueprints/STGPlayerState.STGPlayerState_C|GetHits _asstgplayer_state) (Variables|/Game/Blueprints/STGPlayerState.STGPlayerState_C|GetKills _asstgplayer_state))))
    (:then_1
      (Variables|/Game/UI/HUD.HUD_C|SetHits _hud (Variables|/Game/Blueprints/STGPlayerState.STGPlayerState_C|GetHits _asstgplayer_state)))
    (:then_2
      (Variables|/Game/UI/HUD.HUD_C|SetKills _hud (Variables|/Game/Blueprints/STGPlayerState.STGPlayerState_C|GetKills _asstgplayer_state)))))

(fn ConstructionScript)