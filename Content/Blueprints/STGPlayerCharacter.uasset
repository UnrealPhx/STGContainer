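; Player character for a networked twin-stick shooter, with separate move and fire inputs.
; Tick applies movement and, past a fire deadzone, spawns STGBullets at the RateOfFire interval, faster than the character's max speed.
; Each shot spawns locally, then RequestFireBullet relays it to NotifyFireBullet for non-locally-controlled copies.
; Those copies advance the spawn point by elapsed server time to compensate for latency.
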(event Custom|NotifyFireBullet
  (params (PlayerId :type Integer) (Location :type Vector) (Direction :type Vector) (Speed :type Float%20%28single-precision%29) (Time :type Float%20%28single-precision%29))
  ;[0.1684 1 0.09279] Replicate Bullet Fire Bullet
  (if (not (Pawn|IsLocallyControlled))
    (Game|SpawnActorfromClass "/Game/Blueprints/STGBullet.STGBullet_C" (Math|Transform|MakeTransform (+ Location (* Direction (* Speed (- (GameState|GetServerWorldTimeSeconds (Game|GetGameState)) Time))))) "AlwaysSpawn" 0 Direction Speed 0)))

(event Custom|RequestFireBullet
  (params (PlayerId :type Integer) (Location :type Vector) (Direction :type Vector) (Speed :type Float%20%28single-precision%29) (Time :type Float%20%28single-precision%29))
  (CallFunction|NotifyFireBullet PlayerId Location Direction Speed Time))

(event Collision|EventActorBeginOverlap
  (params (OtherActor :type Actor%20Object%20Reference)))

(event EventTick
  (params (DeltaSeconds :type Float%20%28single-precision%29))
  (bind _charactermovement (Variables|Character|GetCharacterMovement))
  (bind _returnvalue (Class|MovementComponent|GetMaxSpeed _charactermovement))
  (bind _returnvalue_2 (* _returnvalue 1.5))
  (Utilities|FlowControl|Sequence
    (:then_0
      ;[1 1 1] Movement
      (bind _output_get (Variables|Default|SetMove (Math|Vector|MakeVector (Input|AxisValues|GetMoveY) (Input|AxisValues|GetMoveX) 0.0)))
      (bind _output_get_2 (Variables|Default|SetMoveDiretion (Math|Vector|Normalize _output_get)))
      (Pawn|Input|AddMovementInput _output_get_2 (Math|Float|Clamp(Float) (Math|Vector|VectorLengthSquared (Variables|Default|GetMove)) -1.0) false))
    (:then_1
      (bind _output_get_3 (Variables|Default|SetFire (Math|Vector|MakeVector (Input|AxisValues|GetFireY) (Input|AxisValues|GetFireX) 0.0)))
      (Variables|Default|SetFireDiretion (Math|Vector|Normalize _output_get_3))
      (if (>= (Math|Vector|VectorLengthSquared (Variables|Default|GetFire)) 0.25)
        (bind _output_get_4 (Variables|Default|SetLastShot (+ DeltaSeconds (Variables|Default|GetLastShot))))
        (if (>= _output_get_4 (Variables|Default|GetRateOfFire))
          (Variables|Default|SetLastShot 0.0)
          (Game|SpawnActorfromClass "/Game/Blueprints/STGBullet.STGBullet_C" (Math|Transform|MakeTransform (+ (Transformation|GetActorLocation) (* (Variables|Default|GetFireDiretion) 5e+01))) "AlwaysSpawn" 0 (Variables|Default|GetFireDiretion) _returnvalue_2 self)
          (CallFunction|RequestFireBullet (Variables|/Script/Engine.PlayerState|GetPlayerId (Variables|GetPlayerState)) (.Location (Math|Transform|BreakTransform (Math|Transform|MakeTransform (+ (Transformation|GetActorLocation) (* (Variables|Default|GetFireDiretion) 5e+01))))) (Variables|Default|GetFireDiretion) _returnvalue_2 (GameState|GetServerWorldTimeSeconds (Game|GetGameState))))))))

(fn ConstructionScript
  (Variables|Default|SetLastShot (Variables|Default|GetRateOfFire)))