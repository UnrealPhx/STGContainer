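; STGAsteroid_BP is a shootable asteroid that drifts in a random horizontal direction while its instanced mesh spins on yaw each tick.
; The construction script sets velocity and speed on the movement component, then scales size and HP by Difficulty.
; Overlapping STGBullets are destroyed, each costing one HP and crediting a hit to the instigator's STGPlayerState.
; At zero HP it credits a kill and destroys itself with an explosion sound.
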(event EventBeginPlay)

(event Collision|EventActorBeginOverlap
  (params (OtherActor :type Actor%20Object%20Reference))
  (if (Utilities|ClassIsChildOf (Utilities|GetClass OtherActor) "/Game/Blueprints/STGBullet.STGBullet_C")
    (Utilities|FlowControl|Sequence
      (:then_0
        (bind _asstgplayer_character (Utilities|Casting|CastToSTGPlayerCharacter (Game|GetInstigator OtherActor)))
        (bind _asstgplayer_state (Utilities|Casting|CastToSTGPlayerState (Variables|/Script/Engine.Pawn|GetPlayerState _asstgplayer_character))))
      (:then_1
        (Default|UpdateHits _asstgplayer_state 1.0)
        (Audio|PlaySound2D "/Game/Audio/AsteroidHit.AsteroidHit" 1.0 1.0 0.0 "/Game/Audio/Hits.Hits" self))
      (:then_2
        (bind _result (Math|Integer|DecrementInt (Variables|Default|GetHP))
          (:%20%20
            (if (<= _result 0)
              (Default|UpdateKills _asstgplayer_state 1.0)
              (Actor|DestroyActor)
              (Audio|PlaySound2D "/Game/Audio/AsteroidExplode.AsteroidExplode" 1.0 1.0 0.0 "/Game/Audio/Explosions.Explosions" self)))))
      (:then_3
        (Actor|DestroyActor OtherActor)))))

(event EventTick
  (params (DeltaSeconds :type Float%20%28single-precision%29))
  (Transformation|AddLocalRotation (Variables|Default|GetInstancedStaticMesh) (Math|Rotator|MakeRotator 0.0 0.0 (* DeltaSeconds (Variables|Default|GetRotationSpeed))) false false))

(fn ConstructionScript
  (bind _movementcomponent (Variables|Default|GetMovementComponent))
  (bind _difficulty (Variables|Default|GetDifficulty))
  (bind _movementspeed (Variables|Default|GetMovementSpeed))
  (bind _returnvalue (* _difficulty 0.1))
  (bind _returnvalue_2 (+ 1.0 _returnvalue))
  ;[1 1 1] Init Speed & Direction
  (Variables|/Script/Engine.MovementComponent|SetVelocity _movementcomponent (Math|Vector|Normalize (Math|Vector|ProjectVectorontoPlane (Math|Random|RandomUnitVector) "0, 0,1.000000")))
  (Variables|/Script/Engine.ProjectileMovementComponent|SetInitialSpeed _movementcomponent _movementspeed)
  (Variables|/Script/Engine.ProjectileMovementComponent|SetMaxSpeed _movementcomponent _movementspeed)
  ;[1 1 1] Apply Scale for Difficulty
  (Transformation|SetActorScale3D (Math|Vector|MakeVector _returnvalue_2 _returnvalue_2 _returnvalue_2))
  ;[1 1 1] Adjust HP for Difficulty
  (Variables|Default|SetHP (+ (* (Variables|Default|GetDifficulty) (Variables|Default|GetHP)) (Variables|Default|GetHP))))