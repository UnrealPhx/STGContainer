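; STGPlayerState is a player state Blueprint that tracks a player's health, hits and kills and reports changes to the game mode.
; Each update event adjusts its stat (Health is reduced, Hits and Kills are increased), then sends two string events keyed by PlayerName: the change and the new total.
; Events pass through SendPlayerEvent and NotifyCustomEvent, which casts to STGContainerGameModeBase and forwards them, stopping if the cast fails.
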(event Custom|SendPlayerEvent
  (params (Event :type String) (Id :type String) (Value :type String))
  (CallFunction|NotifyCustomEvent Event Id Value))

(event Custom|NotifyCustomEvent
  (params (Event :type String) (Id :type String) (Value :type String))
  (bind _asstgcontainer_game_mode_base (Utilities|Casting|CastToSTGContainerGameModeBase (Game|GetGameMode)))
  (Class|STGContainerGameModeBase|SendPlayerEvent _asstgcontainer_game_mode_base Event Id Value))

(event Custom|UpdateHealth
  (params (Value :type Float%20%28single-precision%29))
  (bind _output_get (Variables|Default|SetHealth (- (Variables|Default|GetHealth) Value)))
  (CallFunction|SendPlayerEvent "Damage" (Variables|Default|GetPlayerName) (Utilities|String|ToString(Float) Value))
  (CallFunction|SendPlayerEvent "Health" (Variables|Default|GetPlayerName) (Utilities|String|ToString(Float) _output_get)))

(event Custom|UpdateKills
  (params (Value :type Float%20%28single-precision%29))
  (bind _output_get (Variables|Default|SetKills (+ (Variables|Default|GetKills) Value)))
  (CallFunction|SendPlayerEvent "Kill" (Variables|Default|GetPlayerName) (Utilities|String|ToString(Float) Value))
  (CallFunction|SendPlayerEvent "Kills" (Variables|Default|GetPlayerName) (Utilities|String|ToString(Float) _output_get)))

(event Custom|UpdateHits
  (params (Value :type Float%20%28single-precision%29))
  (bind _output_get (Variables|Default|SetHits (+ (Variables|Default|GetHits) Value)))
  (CallFunction|SendPlayerEvent "Hit" (Variables|Default|GetPlayerName) (Utilities|String|ToString(Float) Value))
  (CallFunction|SendPlayerEvent "Hits" (Variables|Default|GetPlayerName) (Utilities|String|ToString(Float) _output_get)))

(fn ConstructionScript)